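; BP_stairsound is an actor that plays the Slide_Door3 sound when the player enters or leaves its overlap area.
; Both overlap events compare the other actor to player 0's character, cast to CH_Player, so other actors are ignored.
; The sound plays as non-spatialized 2D audio, with no cooldown or state tracking.
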(event Collision|EventActorBeginOverlap
  (params (OtherActor :type Actor%20Object%20Reference))
  (if (== OtherActor (.AsCH%20Player (Utilities|Casting|CastToCH_Player (Game|GetPlayerCharacter 0))))
    (Audio|PlaySound2D "/Game/Audio/Slide_Door3.Slide_Door3" 1.0 1.0 0.0 0 0)))

(event Collision|EventActorEndOverlap
  (params (OtherActor :type Actor%20Object%20Reference))
  (if (== OtherActor (.AsCH%20Player (Utilities|Casting|CastToCH_Player (Game|GetPlayerCharacter 0))))
    (Audio|PlaySound2D "/Game/Audio/Slide_Door3.Slide_Door3" 1.0 1.0 0.0 0 0)))

(fn ConstructionScript)