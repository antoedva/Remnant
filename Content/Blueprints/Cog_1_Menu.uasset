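; Cog_1_Menu is a spinning cog Blueprint, apparently for the menu, driven by a RotatingMovement component.
; Every Tick sets its rotation rate from RotationSpeed2, dividing pitch by the mesh's world Z scale so larger cogs turn slower, with Reverse flipping the direction.
; The construction script zeroes the rate and sets RotationSpeed, which UpdateRotation merely returns.
; Mesh-clearing and scaling nodes are disconnected.
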(event EventTick
  (params (DeltaSeconds :type Float%20%28single-precision%29))
  (bind _rotationspeed_2 (Variables|Default|GetRotationSpeed_2))
  (bind (_x _y _z) (Math|Vector|BreakVector _rotationspeed_2))
  (if (Variables|Default|GetReverse)
    (Variables|Default|SetRotationDirection -1.0)
    (else
      (Variables|Default|SetRotationDirection 1.0)))
  (Variables|/Script/Engine.RotatingMovementComponent|SetRotationRate (Variables|Components|GetRotatingMovement) (Math|Rotator|MakeRotator _x (|(X*Y) (|(x*y) (|(1/x) (.Z (Math|Vector|BreakVector (Transformation|GetWorldScale (Variables|Components|GetStaticMesh))))) _y) (Variables|Default|GetRotationDirection)) _z))
  (CallFunction|UpdateRotation))

(fn ConstructionScript
  (Variables|/Script/Engine.RotatingMovementComponent|SetRotationRate (Variables|Components|GetRotatingMovement) "0, 0, 0")
  (Variables|Default|SetRotationSpeed "0,20.000000, 0"))

(fn OnRepRotationRate)

(fn UpdateRotation
  (return (Variables|Default|GetRotationSpeed)))