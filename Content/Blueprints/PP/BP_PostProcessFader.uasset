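; Post-process fader that crossfades between present and past looks when the player traverses.
; It starts with the present at full weight and binds to the traverse event on CH_Player's traverse component.
; A FlipFlop plays or reverses the Fade timeline on alternate traversals, driving the PresentPP and PastPP blend weights inversely.
; When the timeline finishes, EffectIndex advances and wraps at EffectNumber, though nothing here applies it.
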(event Custom|OnTraverse
  (Utilities|FlowControl|FlipFlop
    (:A
      (Variables|Default|SetSwitch true)
      (bind _blend (Timeline|Fade PlayFromStart)
        (:Update
          (Utilities|FlowControl|Sequence
            (:then_0
              (Variables|/Script/Engine.PostProcessVolume|SetBlendWeight (Variables|Default|GetPresent%20PP) _blend))
            (:then_1
              (Variables|/Script/Engine.PostProcessVolume|SetBlendWeight (Variables|Default|GetPast%20PP) (- 1.0 _blend)))))
        (:Finished
          (Math|Integer|CompareInt (+ (Variables|Default|GetEffect%20Index) 1) (Variables|Default|GetEffect%20Number)
            (:>
              (Variables|Default|SetEffect%20Index 0 :!label _label))
            (:==
              (goto _label))
            (:<
              (Variables|Default|SetEffect%20Index (+ (Variables|Default|GetEffect%20Index) 1)))))))
    (:B
      (Variables|Default|SetSwitch false)
      (Timeline|Fade ReverseFromEnd))))

(event EventBeginPlay
  (bind _returnvalue (Game|GetPlayerCharacter 0))
  (bind (_asch_player _bsuccess) (Utilities|Casting|CastToCH_Player _returnvalue))
  (Variables|/Script/Engine.PostProcessVolume|SetBlendWeight (Variables|Default|GetPresent%20PP) 1.0)
  (Variables|Default|SetEffect%20Index 2)
  (if _bsuccess
    (bind _returnvalue_2 (Class|FPCharacter|GetTraverseComponent _asch_player))
    (EventDispatchers|BindEventtoOnTraverse _returnvalue_2 (delegate Custom|OnTraverse))))

(fn ConstructionScript)