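; Cog actor that spins through a RotatingMovement component at a configurable RotationSpeed.
; Each tick it sets the rotation rate, dividing the pitch speed by the static mesh's world Z scale so larger cogs turn slower, and flipping pitch when Reverse is set.
; The construction script zeroes the rotation rate, and the OnRep handler for rotation rate is empty.
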(event EventBeginPlay)

(event Collision|EventActorBeginOverlap
  (params (OtherActor :type Actor%20Object%20Reference)))

(event EventTick
  (params (DeltaSeconds :type Float%20%28single-precision%29))
  (bind _rotationspeed (Variables|Default|GetRotationSpeed))
  (bind (_x _y _z) (Math|Vector|BreakVector _rotationspeed))
  (if (Variables|Default|GetReverse)
    (Variables|Default|SetRotationDirection -1.0)
    (else
      (Variables|Default|SetRotationDirection 1.0)))
  (Variables|/Script/Engine.RotatingMovementComponent|SetRotationRate (Variables|Components|GetRotatingMovement) (Math|Rotator|MakeRotator _x (|X*Y (|(x*y) (|1/x (.Z (Math|Vector|BreakVector (Transformation|GetWorldScale (Variables|Components|GetStaticMesh))))) _y) (Variables|Default|GetRotationDirection)) _z)))

(fn ConstructionScript
  (Variables|/Script/Engine.RotatingMovementComponent|SetRotationRate (Variables|Components|GetRotatingMovement) "0, 0, 0"))

(fn OnRepRotationRate)