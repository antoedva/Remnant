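; MultiChannelTestReceiver is a trigger-receiver test actor that shows which of two BlueprintLink channels fired by moving itself vertically.
; BeginPlay caches the actor's starting location and a fixed vertical offset.
; Trigger one moves the actor below that origin and trigger two moves it above, instantly and without sweep, so repeated triggers do not accumulate.
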(event OnTriggerTwo(blueprintLink)
  (Transformation|SetActorLocation (+ (Variables|Default|Getoffset) (Variables|Default|GetoriginalLocation)) false false))

(event OnTriggerOne(blueprintLink)
  (Transformation|SetActorLocation (+ (Math|Vector|NegateVector (Variables|Default|Getoffset)) (Variables|Default|GetoriginalLocation)) false false))

(event EventBeginPlay
  (Variables|Default|SetoriginalLocation (Transformation|GetActorLocation))
  (Variables|Default|Setoffset "0, 0,100.000000"))

(fn ConstructionScript
  (|CallParentFunction))