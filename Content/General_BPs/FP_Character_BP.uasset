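; First-person character Blueprint that places and removes a Clock actor in the world and adds a widget to the viewport on begin play.
; Q line-traces from the camera along the mesh's forward vector, spawns a clock at the hit and calls RenderObjects on it.
; E calls StopRender on the stored clock and destroys it.
; Unwired leftover nodes cover clock detaching, attachment, teleport permission and hard-coded dimension material swapping.
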(event EventBeginPlay
  (bind _returnvalue (UserInterface|CreateWidget "/Game/General_BPs/something.something_C"))
  (UserInterface|Viewport|AddtoViewport _returnvalue 0))

(event Input|KeyboardEvents|Q
  (params (Key :type Key%20Structure))
  (bind _camera (Variables|Default|GetCamera))
  (bind _returnvalue (Transformation|GetWorldLocation _camera))
  (:Pressed
    (bind (_outhit _returnvalue_2) (Collision|LineTraceByChannel _returnvalue (+ _returnvalue (* (Math|Vector|GetForwardVector (Variables|Character|GetMesh)) 5e+02)) "TraceTypeQuery1" false 0 "ForDuration"))
    (if _returnvalue_2
      (bind _returnvalue_3 (Game|SpawnActorfromClass (Variables|Default|GetClockClass) (Math|Conversions|ToTransform(Vector) (.Location (Collision|BreakHitResult _outhit))) "AdjustIfPossibleButAlwaysSpawn" 0 0))
      (bind _output_get (Variables|Default|SetClock _returnvalue_3))
      (Default|RenderObjects _output_get))))

(event Input|KeyboardEvents|E
  (params (Key :type Key%20Structure))
  (bind _clock (Variables|Default|GetClock))
  (:Pressed
    (Default|StopRender _clock)
    (Utilities|IsValid _clock
      (:Is%20Valid
        (Actor|DestroyActor _clock)))))

(fn ConstructionScript)