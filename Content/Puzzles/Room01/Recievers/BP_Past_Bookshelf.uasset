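; BP_Past_Bookshelf is a puzzle receiver for Room01, apparently a bookshelf that slides between preset positions when triggered.
; On BeginPlay it takes the last valid index from the Targets list of receiver target actors.
; BlueprintLink trigger one steps NodeID forward and trigger two steps it back, clamped to that range.
; Each step uses MoveComponentTo to glide the root to that target's location over a few seconds, keeping its rotation.
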(event OnTriggerOne(blueprintLink)
  (if (<= (+ (Variables|Default|GetNode%20ID) 1) (Variables|Default|GetNum%20Nodes))
    (Math|Integer|IncrementInt (Variables|Default|GetNode%20ID)
      (:%20%20
        (Components|MoveComponentTo (Variables|Default|GetDefaultSceneRoot) (Transformation|GetActorLocation (Utilities|Array|Get(acopy) (Variables|/Script/Remnant.ReceiverTargets|Getreceiver_targets_ (Variables|Default|Gettargets_)) (Variables|Default|GetNode%20ID))) (Transformation|GetWorldRotation (Variables|Default|GetDefaultSceneRoot)) false false 3.0 false)))))

(event OnTriggerTwo(blueprintLink)
  (if (>= (- (Variables|Default|GetNode%20ID) 1) 0)
    (Math|Integer|DecrementInt (Variables|Default|GetNode%20ID)
      (:%20%20
        (Components|MoveComponentTo (Variables|Default|GetDefaultSceneRoot) (Transformation|GetActorLocation (Utilities|Array|Get(acopy) (Variables|/Script/Remnant.ReceiverTargets|Getreceiver_targets_ (Variables|Default|Gettargets_)) (Variables|Default|GetNode%20ID))) (Transformation|GetWorldRotation (Variables|Default|GetDefaultSceneRoot)) false false 3.0 false)))))

(event EventBeginPlay
  (bind _output_get (Variables|Default|SetNum%20Nodes (Utilities|Array|Length (Variables|/Script/Remnant.ReceiverTargets|Getreceiver_targets_ (Variables|Default|Gettargets_)))))
  (Math|Integer|DecrementInt _output_get))

(fn ConstructionScript)