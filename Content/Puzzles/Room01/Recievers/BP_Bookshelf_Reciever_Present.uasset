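; Puzzle receiver for the Room01 present-day bookshelf that moves along a list of target actors.
; Each BlueprintLink trigger increments a node index and, while it stays within the list, slides the root component to that target's location over two seconds, keeping its rotation.
; BeginPlay caches the last valid index from the receiver target list, so triggers past the final node cause no movement.
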(event OnTrigger(blueprintLink)
  (bind _node_id (Variables|Default|GetNode%20ID))
  (Math|Integer|IncrementInt _node_id
    (:%20%20
      (if (<= _node_id (Variables|Default|GetNum%20Nodes))
        (Components|MoveComponentTo (Variables|Default|GetDefaultSceneRoot) (Transformation|GetActorLocation (Utilities|Array|Get(acopy) (Variables|/Script/Remnant.ReceiverTargets|Getreceiver_targets_ (Variables|Default|Gettargets_)) (Variables|Default|GetNode%20ID))) (Transformation|GetWorldRotation (Variables|Default|GetDefaultSceneRoot)) false false 2.0 false)))))

(event EventBeginPlay
  (bind _output_get (Variables|Default|SetNum%20Nodes (Utilities|Array|Length (Variables|/Script/Remnant.ReceiverTargets|Getreceiver_targets_ (Variables|Default|Gettargets_)))))
  (Math|Integer|DecrementInt _output_get))

(fn ConstructionScript
  (|CallParentFunction))