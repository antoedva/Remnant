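; One-shot button for part three of the Room01 machine puzzle that starts the past and present sequence switches.
; On trigger, it moves each sequence trigger onto its matching receiver, calling Start on both switches before and after the move.
; It also moves both lever triggers to a marker actor, then slides its mesh a short way to show the press.
; Despite the ResetButton name, a flag blocks any further presses.
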(event OnTrigger(triggerComponent)
  (if (not (Variables|Default|GetBeenTriggered))
    (CallFunction|StartSequenceMachine)
    (CallFunction|PositionLeverTriggers)
    (Variables|Default|SetBeenTriggered true)
    (Components|MoveComponentTo (Variables|Default|GetStaticMesh) (+ (Variables|Default|GetOriginalLocation) "10.000000, 0, 0") "0, 0, 0" false false 0.5 false)))

(event EventBeginPlay
  (Variables|Default|SetOriginalLocation (Math|Transform|TransformLocation (Transformation|GetRelativeTransform (Variables|Default|GetStaticMesh)) "0, 0, 0"))
  (Variables|Default|SetBeenTriggered false))

(fn ConstructionScript)

(fn StartSequenceMachine
  (bind _assequence_switch (Utilities|Casting|CastToSequenceSwitch (Variables|Default|GetSequenceReceiverPresent)))
  (Default|Start _assequence_switch)
  (bind _assequence_switch_2 (Utilities|Casting|CastToSequenceSwitch (Variables|Default|GetSequenceReceiverPast)))
  (Default|Start _assequence_switch_2)
  (Transformation|SetActorLocation (Variables|Default|GetSequenceTriggerPresent) (Transformation|GetActorLocation (Variables|Default|GetSequenceReceiverPresent)) false false)
  (Transformation|SetActorLocation (Variables|Default|GetSequenceTriggerPast) (Transformation|GetActorLocation (Variables|Default|GetSequenceReceiverPast)) false false)
  (bind _assequence_switch_3 (Utilities|Casting|CastToSequenceSwitch (Variables|Default|GetSequenceReceiverPresent)))
  (Default|Start _assequence_switch_3)
  (bind _assequence_switch_4 (Utilities|Casting|CastToSequenceSwitch (Variables|Default|GetSequenceReceiverPast)))
  (Default|Start _assequence_switch_4)
  (return))

(fn PositionLeverTriggers
  (bind _leverlocationactor (Variables|Default|GetLeverLocationActor))
  (bind _returnvalue (Transformation|GetActorLocation _leverlocationactor))
  (Transformation|SetActorLocation (Variables|Default|GetLeverTriggerPast) _returnvalue false false)
  (Transformation|SetActorLocation (Variables|Default|GetLeverTriggerPresent) _returnvalue false false)
  (return))