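; BP_TriggerDoorOpener is the button trigger for part 04 of the Room01 machine puzzle, named as a door opener though it holds no door logic.
; BeginPlay caches the button's relative transform and creates dynamic materials for the button and bottom plate.
; When TriggerComponent fires OnTrigger, the button slides inward along local X, both materials' "Activated" parameter drops to zero, and SphereComponent is deactivated.
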(event OnTrigger(triggerComponent)
  (Components|MoveComponentTo (Variables|Default|GetActualButton) (+ (Variables|Default|GetButtonOriginalLocation) "-10.000000,0.000000,0.000000") (Variables|Default|GetButtonOriginalRotation) false false 0.3 false)
  (Rendering|Material|SetScalarParameterValue (Variables|Default|GetDynamicMaterialInstanceBottom) "Activated" 0.0 :!class /Script/Engine.MaterialInstanceDynamic)
  (Rendering|Material|SetScalarParameterValue (Variables|Default|GetDynamicMaterialInstanceActualButton) "Activated" 0.0 :!class /Script/Engine.MaterialInstanceDynamic)
  (Components|Activation|Deactivate (Variables|Default|GetsphereComponent)))

(event EventBeginPlay
  (bind _actualbutton (Variables|Default|GetActualButton))
  (bind _actualbutton_2 (Variables|Default|GetActualButton))
  (bind _bottomplate (Variables|Default|GetBottomPlate))
  (bind _returnvalue (Transformation|GetRelativeTransform _actualbutton))
  (bind (_location _rotation) (Math|Transform|BreakTransform _returnvalue))
  (Variables|Default|SetButtonOriginalLocation _location)
  (Variables|Default|SetButtonOriginalRotation _rotation)
  (bind _returnvalue_2 (Rendering|Material|CreateDynamicMaterialInstance _bottomplate 0 (Rendering|Material|GetMaterial _bottomplate 0) "None" :!class /Script/Engine.PrimitiveComponent))
  (Variables|Default|SetDynamicMaterialInstanceBottom _returnvalue_2)
  (bind _returnvalue_3 (Rendering|Material|CreateDynamicMaterialInstance _actualbutton_2 0 (Rendering|Material|GetMaterial _actualbutton_2 0) "None" :!class /Script/Engine.PrimitiveComponent))
  (Variables|Default|SetDynamicMaterialInstanceActualButton _returnvalue_3))

(fn ConstructionScript)