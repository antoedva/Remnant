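; BP_SequenceStarter is a trigger Blueprint in part four of Room01's machine puzzle, currently with no active behavior.
; Its TriggerComponent OnTrigger event is empty, and the construction script does nothing.
; A disconnected graph would flip-flop between two Targets and briefly tween SphereComponent to the selected target's rotation.
; That unused move feeds the sphere's world location into a relative-location target.
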(event OnTrigger(triggerComponent))

(fn ConstructionScript)