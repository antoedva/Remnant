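; BP_DoorOpener_PRESENT is a button actor for Part04 of the Room01 machine puzzle that visually presses down when triggered.
; It caches the ActualButton component's relative location and rotation on BeginPlay.
; An OnTrigger event from BlueprintLink eases the button down along local Z with MoveComponentTo, keeping its rotation.
; The graph contains no door logic and never raises the button again.
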(event OnTrigger(blueprintLink)
  (params (channel :type Integer))
  (Components|MoveComponentTo (Variables|Default|GetActualButton) (+ (Variables|Default|GetButtonOriginalLocation) "0,0.000000,-10.000000") (Variables|Default|GetButtonOriginalRotation) false false 0.3 false))

(event EventBeginPlay
  (bind _actualbutton (Variables|Default|GetActualButton))
  (bind _returnvalue (Transformation|GetRelativeTransform _actualbutton))
  (bind (_location _rotation) (Math|Transform|BreakTransform _returnvalue))
  (Variables|Default|SetButtonOriginalLocation _location)
  (Variables|Default|SetButtonOriginalRotation _rotation))

(fn ConstructionScript)