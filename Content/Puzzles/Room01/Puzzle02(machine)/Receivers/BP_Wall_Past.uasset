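; BP_Wall_Past is a puzzle receiver wall for the machine puzzle in Room 01, moved when the linked trigger fires.
; On channel 0 of its BlueprintLink trigger event, it slides its root component over five seconds to the location of the first receiver target actor.
; Only location is used; the target's rotation is read but left unconnected.
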(event OnTrigger(blueprintLink)
  (params (channel :type Integer))
  (switch int channel
    (:0
      (Components|MoveComponentTo (Variables|Default|GetDefaultSceneRoot) (Transformation|GetActorLocation (Utilities|Array|Get(acopy) (Variables|/Script/Remnant.ReceiverTargets|Getreceiver_targets_ (Variables|Default|Gettargets_)))) "0, 0, 0" false false 5.0 false))))

(fn ConstructionScript)