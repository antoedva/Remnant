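; Puzzle receiver for the present-time whale in the Room01 machine puzzle, which steps along a list of target nodes.
; BlueprintLink triggers on channel 2 advance the node index and channel 3 move it back, clamped to the ends of Targets.ReceiverTargets.
; Each successful step snaps the scene root to that node actor's location without sweep or interpolation.
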(event OnTrigger(blueprintLink)
  (params (channel :type Integer))
  (switch int channel
    (:2
      (if (CallFunction|IncrementID)
        (Transformation|SetRelativeLocation (Variables|Default|GetDefaultSceneRoot) (Transformation|GetActorLocation (Utilities|GetNodeID)) false false)))
    (:3
      (if (CallFunction|DecrementID)
        (Transformation|SetRelativeLocation (Variables|Default|GetDefaultSceneRoot) (Transformation|GetActorLocation (Utilities|GetNodeID)) false false)))))

(event EventBeginPlay
  (bind _output_get (Variables|Default|SetNum%20Nodes (Utilities|Array|Length (Variables|/Script/Remnant.ReceiverTargets|Getreceiver_targets_ (Variables|Default|Gettargets_)))))
  (Math|Integer|DecrementInt _output_get))

(fn ConstructionScript)

(fn IncrementID
  (if (<= (+ (Variables|Default|GetNode%20ID) 1) (Variables|Default|GetNum%20Nodes))
    (Math|Integer|IncrementInt (Variables|Default|GetNode%20ID)
      (:%20%20
        (return true)))
    (else
      (return false))))

(fn DecrementID
  (if (>= (- (Variables|Default|GetNode%20ID) 1) 0)
    (Math|Integer|DecrementInt (Variables|Default|GetNode%20ID)
      (:%20%20
        (return true)))
    (else
      (return false))))