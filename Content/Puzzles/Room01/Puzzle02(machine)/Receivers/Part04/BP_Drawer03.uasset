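; BP_Drawer03 is a drawer receiver for the Room01 machine puzzle that makes a timed out-and-back move between target actors.
; A BlueprintLink trigger on channel 0 starts a delay, then slides the root component to the next node's location, keeping its rotation.
; After a short pause it steps back to the previous node.
; IncrementID and DecrementID bounds-check the node index against the ReceiverTargets list.
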(event OnTrigger(blueprintLink)
  (params (channel :type Integer))
  (switch int channel
    (:0
      (Utilities|FlowControl|Delay 1e+01)
      (if (CallFunction|IncrementID)
        (Components|MoveComponentTo (Variables|Default|GetDefaultSceneRoot) (Transformation|GetActorLocation (Utilities|GetNodeID)) (Transformation|GetWorldRotation (Variables|Default|GetDefaultSceneRoot)) false false 3.0 false)
        (Utilities|FlowControl|Delay 2.0)
        (if (CallFunction|DecrementID)
          (Components|MoveComponentTo (Variables|Default|GetDefaultSceneRoot) (Transformation|GetActorLocation (Utilities|GetNodeID)) (Transformation|GetWorldRotation (Variables|Default|GetDefaultSceneRoot)) false false 3.0 false))))))

(event EventBeginPlay
  (bind _output_get (Variables|Default|SetNum%20Nodes (Utilities|Array|Length (Variables|/Script/Remnant.ReceiverTargets|Getreceiver_targets_ (Variables|Default|Gettargets_)))))
  (Math|Integer|DecrementInt _output_get))

(fn ConstructionScript)

(fn IncrementID
  (if (<= (+ (Variables|Default|GetNode%20ID) 1) (Variables|Default|GetNum%20Nodes))
    (Math|Integer|IncrementInt (Variables|Default|GetNode%20ID)
      (:%20%20
        (return true)))
    (else
      (return false))))

(fn DecrementID
  (if (>= (- (Variables|Default|GetNode%20ID) 1) 0)
    (Math|Integer|DecrementInt (Variables|Default|GetNode%20ID)
      (:%20%20
        (return true)))
    (else
      (return false))))