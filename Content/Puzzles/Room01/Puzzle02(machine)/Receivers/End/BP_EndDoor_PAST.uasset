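; End door receiver for the Room01 machine puzzle (PAST variant) that swings open when triggered.
; On BeginPlay it caches the root component's relative transform and sets a yaw offset.
; The BlueprintLink OnTrigger event uses MoveComponentTo to quickly rotate the root to that offset from its initial yaw, with no logic to close it again.
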(event OnTrigger(blueprintLink)
  (params (channel :type Integer))
  (bind _initialrotation (Variables|Default|GetInitialRotation))
  (Components|MoveComponentTo (Variables|Default|GetDefaultSceneRoot) (Variables|Default|GetInitialLocation) (Math|Rotator|MakeRotator (.roll _initialrotation) (.pitch _initialrotation) (+ (.yaw _initialrotation) (Variables|Default|GetRotationOffset))) false false 0.2 false))

(event EventBeginPlay
  (bind _defaultsceneroot (Variables|Default|GetDefaultSceneRoot))
  (bind _returnvalue (Transformation|GetRelativeTransform _defaultsceneroot))
  (bind (_location _rotation) (Math|Transform|BreakTransform _returnvalue))
  (Variables|Default|SetRotationOffset 85.0)
  (Variables|Default|SetInitialLocation _location)
  (Variables|Default|SetInitialRotation _rotation))

(fn ConstructionScript)