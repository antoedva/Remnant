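; Past-era bookshelf receiver for the Room01 puzzle that slides between target nodes and controls which version of a key is in place.
; BlueprintLink channels 0 and 1 step the node index forward or back within bounds, then move the shelf over a few seconds.
; At node 1, treated as the middle, the floor key is restored and the glass-encased key is parked at world origin; elsewhere they swap, as the move starts.
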(event OnTrigger(blueprintLink)
  (params (channel :type Integer))
  (switch int channel
    (:0
      (if (CallFunction|IncrementID)
        (bind _boolreturn (CallFunction|IsBookshelfinMiddle))
        (if _boolreturn
          (CallFunction|MakeKeyAvailable)
          (else
            (CallFunction|MakeKeyNotAvailable)))
        (Components|MoveComponentTo (Variables|Default|GetDefaultSceneRoot) (Transformation|GetActorLocation (Utilities|GetNodeID)) (Transformation|GetWorldRotation (Variables|Default|GetDefaultSceneRoot)) false false 3.0 false)))
    (:1
      (if (CallFunction|DecrementID)
        (bind _boolreturn_2 (CallFunction|IsBookshelfinMiddle))
        (if _boolreturn_2
          (CallFunction|MakeKeyAvailable)
          (else
            (CallFunction|MakeKeyNotAvailable)))
        (Components|MoveComponentTo (Variables|Default|GetDefaultSceneRoot) (Transformation|GetActorLocation (Utilities|GetNodeID)) (Transformation|GetWorldRotation (Variables|Default|GetDefaultSceneRoot)) false false 3.0 false)))))

(event EventBeginPlay
  (bind _output_get (Variables|Default|SetNum%20Nodes (Utilities|Array|Length (Variables|/Script/Remnant.ReceiverTargets|Getreceiver_targets_ (Variables|Default|Gettargets_)))))
  (Math|Integer|DecrementInt _output_get
    (:%20%20
      (Variables|Default|SetFloorKeyOriginalLocation (Transformation|GetActorLocation (Variables|Default|GetKeyOnFloor)))
      (Variables|Default|SetGlassKeyOriginalLocation (Transformation|GetActorLocation (Variables|Default|GetKeyInsideGlass)))
      (CallFunction|MakeKeyNotAvailable))))

(fn ConstructionScript)

(fn DecrementID
  (if (>= (- (Variables|Default|GetNode%20ID) 1) 0)
    (Math|Integer|DecrementInt (Variables|Default|GetNode%20ID)
      (:%20%20
        (return true)))
    (else
      (return false))))

(fn IncrementID
  (if (<= (+ (Variables|Default|GetNode%20ID) 1) (Variables|Default|GetNum%20Nodes))
    (Math|Integer|IncrementInt (Variables|Default|GetNode%20ID)
      (:%20%20
        (return true)))
    (else
      (return false))))

(fn MakeKeyAvailable
  (Transformation|SetActorLocation (Variables|Default|GetKeyInsideGlass) "0, 0, 0" false false)
  (Transformation|SetActorLocation (Variables|Default|GetKeyOnFloor) (Variables|Default|GetFloorKeyOriginalLocation) false false)
  (return))

(fn MakeKeyNotAvailable
  (Transformation|SetActorLocation (Variables|Default|GetKeyOnFloor) "0, 0, 0" false false)
  (Transformation|SetActorLocation (Variables|Default|GetKeyInsideGlass) (Variables|Default|GetGlassKeyOriginalLocation) false false)
  (return))

(fn IsBookshelfinMiddle
  (if (== (Variables|Default|GetNode%20ID) 1)
    (return true)
    (else
      (return false))))