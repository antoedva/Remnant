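; Tutorial-room present button that moves a sphere between two reference actors when triggered.
; On BeginPlay it creates a dynamic material on its static mesh and zeroes the emissive intensity, which nothing here raises.
; On trigger, latent moves send SphereComponent to StartActor's transform, then after a short delay to EndActor's.
; Both moves pass world locations and rotations as relative targets.
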(event OnTrigger(triggerComponent)
  (bind _start_actor (Variables|Default|GetStart%20Actor))
  (bind _end_actor (Variables|Default|GetEnd%20Actor))
  (Utilities|FlowControl|Sequence
    (:then_1
      (Components|MoveComponentTo (Variables|Default|GetsphereComponent) (Transformation|GetActorLocation _start_actor) (Transformation|GetActorRotation _start_actor) false false 0.2 false)
      (Utilities|FlowControl|Delay 0.5)
      (Components|MoveComponentTo (Variables|Default|GetsphereComponent) (Transformation|GetActorLocation _end_actor) (Transformation|GetActorRotation _end_actor) false false 0.2 false))))

(event EventBeginPlay
  (bind _staticmesh (Variables|Default|GetStaticMesh))
  (bind _returnvalue (Rendering|Material|CreateDynamicMaterialInstance _staticmesh 0 (Rendering|Material|GetMaterial _staticmesh 0) "None" :!class /Script/Engine.PrimitiveComponent))
  (Rendering|Material|SetScalarParameterValue _returnvalue "Emissive_intensity" 0.0 :!class /Script/Engine.MaterialInstanceDynamic))

(fn ConstructionScript)