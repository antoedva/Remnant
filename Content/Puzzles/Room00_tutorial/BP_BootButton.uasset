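; Boot button for the tutorial puzzle room that, when triggered, opens the All_Combined level.
; BeginPlay creates a dynamic material with its glow off and reuses or creates the loading screen widget cached on the game instance, keeping it hidden.
; Triggering lights the button, plays a sound and moves a sphere component to a start actor, then an end actor, before dimming, showing the loading screen and opening the level.
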(event OnTrigger(triggerComponent)
  (bind _start_actor (Variables|Default|GetStart%20Actor))
  (bind _end_actor (Variables|Default|GetEnd%20Actor))
  (Utilities|FlowControl|Sequence
    (:then_0
      (Rendering|Material|SetScalarParameterValue (Variables|Default|GetDynamicMat) "Emissive_intensity" 3e+01 :!class /Script/Engine.MaterialInstanceDynamic))
    (:then_1
      (Audio|PlaySound2D "/Game/Audio/Sounds/Intractibles/Button.Button" 1.0 1.0 0.0 0 0)
      (Components|MoveComponentTo (Variables|Default|GetsphereComponent) (Transformation|GetActorLocation _start_actor) (Transformation|GetActorRotation _start_actor) false false 0.2 false)
      (Utilities|FlowControl|Delay 0.5)
      (Components|MoveComponentTo (Variables|Default|GetsphereComponent) (Transformation|GetActorLocation _end_actor) (Transformation|GetActorRotation _end_actor) false false 0.2 false)
      (Rendering|Material|SetScalarParameterValue (Variables|Default|GetDynamicMat) "Emissive_intensity" 0.0 :!class /Script/Engine.MaterialInstanceDynamic)
      (Widget|SetVisibility (Variables|Default|GetLoadingScreen) "Visible")
      (Utilities|FlowControl|Delay 0.2)
      (Game|OpenLevel(byName) "All_Combined"))))

(event EventBeginPlay
  (bind _returnvalue (Game|GetGameInstance))
  (bind _staticmesh (Variables|Default|GetStaticMesh))
  (bind _asbp_remnant_gi (Utilities|Casting|CastToBP_Remnant_GI _returnvalue))
  (bind _returnvalue_2 (Rendering|Material|CreateDynamicMaterialInstance _staticmesh 0 (Rendering|Material|GetMaterial _staticmesh 0) "None" :!class /Script/Engine.PrimitiveComponent))
  (bind _output_get (Variables|Default|SetDynamicMat _returnvalue_2))
  (Rendering|Material|SetScalarParameterValue _output_get "Emissive_intensity" 0.0 :!class /Script/Engine.MaterialInstanceDynamic)
  (Utilities|IsValid (Variables|/Game/Instance/BP_Remnant_GI.BP_Remnant_GI_C|GetLoadingWidget _asbp_remnant_gi)
    (:Is%20Valid
      (Variables|Default|SetLoadingScreen (Variables|/Game/Instance/BP_Remnant_GI.BP_Remnant_GI_C|GetLoadingWidget _asbp_remnant_gi)))
    (:Is%20Not%20Valid
      (bind _returnvalue_3 (UserInterface|CreateWidget "/Game/UI/Menu/LoadingScreen/BP_LoadingScreen.BP_LoadingScreen_C"))
      (bind _output_get_2 (Variables|/Game/Instance/BP_Remnant_GI.BP_Remnant_GI_C|SetLoadingWidget _asbp_remnant_gi _returnvalue_3))
      (bind _output_get_3 (Variables|Default|SetLoadingScreen _output_get_2))))
  (UserInterface|Viewport|AddtoViewport _output_get_3 0)
  (Widget|SetVisibility _output_get_3 "Hidden"))

(fn ConstructionScript)