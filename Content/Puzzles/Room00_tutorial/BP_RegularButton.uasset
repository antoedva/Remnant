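; Button Blueprint for the tutorial puzzle room that moves its sphere component between two reference actors when triggered.
; The trigger component's OnTrigger event moves the sphere to StartActor's location and rotation, waits briefly, then moves it to EndActor's.
; Both moves use MoveComponentTo, feeding the actors' world transforms into its relative-space targets.
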(event OnTrigger(triggerComponent)
  (bind _start_actor (Variables|Default|GetStart%20Actor))
  (bind _end_actor (Variables|Default|GetEnd%20Actor))
  (Components|MoveComponentTo (Variables|Default|GetsphereComponent) (Transformation|GetActorLocation _start_actor) (Transformation|GetActorRotation _start_actor) false false 0.2 false)
  (Utilities|FlowControl|Delay 0.5)
  (Components|MoveComponentTo (Variables|Default|GetsphereComponent) (Transformation|GetActorLocation _end_actor) (Transformation|GetActorRotation _end_actor) false false 0.2 false))

(fn ConstructionScript)