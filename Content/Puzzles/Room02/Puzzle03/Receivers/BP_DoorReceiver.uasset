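; Puzzle receiver that moves its root component between TargetUp and TargetDown actors, driven by BlueprintLink channels and ascend/descend dispatchers.
; Channel 0 trigger and reverse start upward or downward movement, while channels 10 and 11 freeze and unfreeze it, checking PressurePlate00 occupancy on unfreeze.
; Timelines track elapsed time so MoveComponentTo covers the remainder of a three-second travel, with DoOnce gates reset when movement stops or completes.
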(event OnTrigger(blueprintLink)
  (params (channel :type Integer))
  (switch int channel
    (:0
      (if (not (Variables|Default|GetFrozen))
        (Default|CallAscendStairs)))
    (:10
      (Variables|Default|SetFrozen true)
      (Utilities|FlowControl|Sequence :!label _label
        (:then_0
          (bind _elapsed_time (Timeline|Timeline_0 Stop)
            (:Update
              (Variables|Default|SetElapsedTime _elapsed_time)
              (Utilities|FlowControl|DoOnce false :!label _label_2
                (:Completed
                  (Components|MoveComponentTo (Variables|Default|GetDefaultSceneRoot) (Transformation|GetActorLocation (Variables|Default|GetTargetUp)) (Transformation|GetWorldRotation (Variables|Default|GetDefaultSceneRoot)) false false (- 3.0 (Variables|Default|GetElapsedTime)) false :!label _label_3)
                  (goto _label_2 Reset))))))
        (:then_1
          (goto _label_2 Reset))
        (:then_2
          (goto _label_3 Stop))))
    (:11
      (Variables|Default|SetFrozen false)
      (if (CallFunction|ActoronPlate)
        (goto _label)
        (else
          (bind _elapsed_time_2 (Timeline|Timeline_1 Play)
            (:Update
              (Variables|Default|SetElapsedTime _elapsed_time_2)
              (Utilities|FlowControl|DoOnce false :!label _label_4
                (:Completed
                  (Components|MoveComponentTo (Variables|Default|GetDefaultSceneRoot) (Transformation|GetActorLocation (Variables|Default|GetTargetDown)) (Transformation|GetWorldRotation (Variables|Default|GetDefaultSceneRoot)) false false (- 3.0 (Variables|Default|GetElapsedTime)) false)
                  (goto _label_4 Reset))))))))))

(event OnTriggerReverse(blueprintLink)
  (params (channel :type Integer))
  (switch int channel
    (:0
      (if (not (Variables|Default|GetFrozen))
        (Utilities|FlowControl|Sequence
          (:then_0
            (Utilities|FlowControl|Sequence
              (:then_0
                (bind _elapsed_time (Timeline|Timeline_0 Stop)
                  (:Update
                    (Variables|Default|SetElapsedTime _elapsed_time)
                    (Utilities|FlowControl|DoOnce false :!label _label
                      (:Completed
                        (Components|MoveComponentTo (Variables|Default|GetDefaultSceneRoot) (Transformation|GetActorLocation (Variables|Default|GetTargetUp)) (Transformation|GetWorldRotation (Variables|Default|GetDefaultSceneRoot)) false false (- 3.0 (Variables|Default|GetElapsedTime)) false :!label _label_2)
                        (goto _label Reset))))))
              (:then_1
                (goto _label Reset))
              (:then_2
                (goto _label_2 Stop))))
          (:then_1
            (Default|CallDescendStairs)))))
    (:10
      (Variables|Default|SetFrozen true)
      (Utilities|FlowControl|Sequence
        (:then_0
          (bind _elapsed_time_2 (Timeline|Timeline_1 Stop)
            (:Update
              (Variables|Default|SetElapsedTime _elapsed_time_2)
              (Utilities|FlowControl|DoOnce false :!label _label_3
                (:Completed
                  (Components|MoveComponentTo (Variables|Default|GetDefaultSceneRoot) (Transformation|GetActorLocation (Variables|Default|GetTargetDown)) (Transformation|GetWorldRotation (Variables|Default|GetDefaultSceneRoot)) false false (- 3.0 (Variables|Default|GetElapsedTime)) false :!label _label_4)
                  (goto _label_3 Reset))))))
        (:then_1
          (goto _label_3 Reset))
        (:then_2
          (goto _label_4 Stop))))
    (:11
      (Variables|Default|SetFrozen false)
      (if (CallFunction|ActoronPlate)
        (Timeline|Timeline_0 Play)
        (else
          (Timeline|Timeline_1 PlayFromStart))))))

(event Custom|On%20AscendStairs
  (Utilities|FlowControl|Sequence
    (:then_0
      (Utilities|FlowControl|Sequence
        (:then_0
          (bind _elapsed_time (Timeline|Timeline_1 Stop)
            (:Update
              (Variables|Default|SetElapsedTime _elapsed_time)
              (Utilities|FlowControl|DoOnce false :!label _label
                (:Completed
                  (Components|MoveComponentTo (Variables|Default|GetDefaultSceneRoot) (Transformation|GetActorLocation (Variables|Default|GetTargetDown)) (Transformation|GetWorldRotation (Variables|Default|GetDefaultSceneRoot)) false false (- 3.0 (Variables|Default|GetElapsedTime)) false :!label _label_2)
                  (goto _label Reset))))))
        (:then_1
          (goto _label Reset))
        (:then_2
          (goto _label_2 Stop))))
    (:then_1
      (bind _elapsed_time_2 (Timeline|Timeline_0 PlayFromStart)
        (:Update
          (Variables|Default|SetElapsedTime _elapsed_time_2)
          (Utilities|FlowControl|DoOnce false :!label _label_3
            (:Completed
              (Components|MoveComponentTo (Variables|Default|GetDefaultSceneRoot) (Transformation|GetActorLocation (Variables|Default|GetTargetUp)) (Transformation|GetWorldRotation (Variables|Default|GetDefaultSceneRoot)) false false (- 3.0 (Variables|Default|GetElapsedTime)) false)
              (goto _label_3 Reset))))))))

(event Custom|On%20DescendStairs
  (bind _elapsed_time (Timeline|Timeline_1 PlayFromStart)
    (:Update
      (Variables|Default|SetElapsedTime _elapsed_time)
      (Utilities|FlowControl|DoOnce false :!label _label
        (:Completed
          (Components|MoveComponentTo (Variables|Default|GetDefaultSceneRoot) (Transformation|GetActorLocation (Variables|Default|GetTargetDown)) (Transformation|GetWorldRotation (Variables|Default|GetDefaultSceneRoot)) false false (- 3.0 (Variables|Default|GetElapsedTime)) false)
          (goto _label Reset))))))

(event EventBeginPlay
  (EventDispatchers|BindEventtoAscendStairs (delegate Custom|On%20AscendStairs))
  (EventDispatchers|BindEventtoDescendStairs (delegate Custom|On%20DescendStairs)))

(fn ConstructionScript)

(fn ActoronPlate
  (return (Class|VolumeTriggerActor|IsActorInsideVolume (Variables|Default|GetPressurePlate00))))