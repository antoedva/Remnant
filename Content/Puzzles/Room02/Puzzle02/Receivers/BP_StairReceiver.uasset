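; Puzzle stair receiver that raises toward TargetUp when both pressure plates are occupied and lowers toward TargetDown otherwise, driven by BlueprintLink channel triggers.
; Separate channels freeze and resume motion, with an Ascending flag limiting freeze handling of descents.
; Timelines track elapsed time for DoOnce-gated MoveComponentTo calls, so resumed moves use only the remainder of the three-second travel.
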(event OnTrigger(blueprintLink)
  (params (channel :type Integer))
  (switch int channel
    (:0
      (if (not (Variables|Default|GetFrozen))
        (if (CallFunction|BothPlatesActive)
          (Default|CallAscendStairs))))
    (:10
      (Variables|Default|SetFrozen true)
      (Utilities|FlowControl|Sequence
        (:then_0
          (bind _elapsed_time (Timeline|Timeline_0 Stop)
            (:Update
              (Variables|Default|SetElapsedTime _elapsed_time)
              (Utilities|FlowControl|DoOnce false :!label _label
                (:Completed
                  (Components|MoveComponentTo (Variables|Default|GetDefaultSceneRoot) (Transformation|GetActorLocation (Variables|Default|GetTargetUp)) (Transformation|GetWorldRotation (Variables|Default|GetDefaultSceneRoot)) false false (- 3.0 (Variables|Default|GetElapsedTime)) false :!label _label_2)
                  (Utilities|FlowControl|Sequence
                    (:then_0
                      (goto _label Reset))
                    (:then_1
                      (if (not (Variables|Default|GetFrozen))
                        (Variables|Default|SetAscending false)))))))))
        (:then_1
          (goto _label Reset))
        (:then_2
          (goto _label_2 Stop))))
    (:11
      (Variables|Default|SetFrozen false)
      (Timeline|Timeline_0 Play))))

(event OnTriggerReverse(blueprintLink)
  (params (channel :type Integer))
  (bind _ascending (Variables|Default|GetAscending))
  (switch int channel
    (:0
      (if (not (Variables|Default|GetFrozen))
        (if (not (CallFunction|BothPlatesActive))
          (Default|CallDescendStairs))))
    (:10
      (Variables|Default|SetFrozen true)
      (if (not _ascending)
        (Utilities|FlowControl|Sequence
          (:then_0
            (bind _elapsed_time (Timeline|Timeline_1 Stop)
              (:Update
                (Variables|Default|SetElapsedTime _elapsed_time)
                (Utilities|FlowControl|DoOnce false :!label _label
                  (:Completed
                    (Components|MoveComponentTo (Variables|Default|GetDefaultSceneRoot) (Transformation|GetActorLocation (Variables|Default|GetTargetDown)) (Transformation|GetWorldRotation (Variables|Default|GetDefaultSceneRoot)) false false (- 3.0 (Variables|Default|GetElapsedTime)) false :!label _label_2)
                    (goto _label Reset))))))
          (:then_1
            (goto _label Reset))
          (:then_2
            (goto _label_2 Stop)))))
    (:11
      (Variables|Default|SetFrozen false)
      (if (not _ascending)
        (Timeline|Timeline_1 Play)))))

(event Custom|On%20AscendStairs
  (Variables|Default|SetAscending true)
  (bind _elapsed_time (Timeline|Timeline_0 PlayFromStart)
    (:Update
      (Variables|Default|SetElapsedTime _elapsed_time)
      (Utilities|FlowControl|DoOnce false :!label _label
        (:Completed
          (Components|MoveComponentTo (Variables|Default|GetDefaultSceneRoot) (Transformation|GetActorLocation (Variables|Default|GetTargetUp)) (Transformation|GetWorldRotation (Variables|Default|GetDefaultSceneRoot)) false false (- 3.0 (Variables|Default|GetElapsedTime)) false)
          (Utilities|FlowControl|Sequence
            (:then_0
              (goto _label Reset))
            (:then_1
              (if (not (Variables|Default|GetFrozen))
                (Variables|Default|SetAscending false)))))))))

(event Custom|On%20DescendStairs
  (bind _elapsed_time (Timeline|Timeline_1 PlayFromStart)
    (:Update
      (Variables|Default|SetElapsedTime _elapsed_time)
      (Utilities|FlowControl|DoOnce false :!label _label
        (:Completed
          (Components|MoveComponentTo (Variables|Default|GetDefaultSceneRoot) (Transformation|GetActorLocation (Variables|Default|GetTargetDown)) (Transformation|GetWorldRotation (Variables|Default|GetDefaultSceneRoot)) false false (- 3.0 (Variables|Default|GetElapsedTime)) false)
          (goto _label Reset))))))

(event EventBeginPlay
  (EventDispatchers|BindEventtoAscendStairs (delegate Custom|On%20AscendStairs))
  (EventDispatchers|BindEventtoDescendStairs (delegate Custom|On%20DescendStairs)))

(fn ConstructionScript)

(fn BothPlatesActive
  (return (and (Class|VolumeTriggerActor|IsActorInsideVolume (Variables|Default|GetPressurePlate01)) (Class|VolumeTriggerActor|IsActorInsideVolume (Variables|Default|GetPressurePlate00)))))