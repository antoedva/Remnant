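; BP_PressurePlateTrigger is a puzzle pressure plate that sinks when triggered and rises when the trigger reverses.
; TriggerComponent's OnTrigger and OnTriggerReverse events each play a 2D press or release sound.
; Each event stops the opposing MoveComponentTo, then eases CollisionComponent toward the TargetDown or TargetUp actor's location over a short fixed time.
; World locations and rotation feed the relative-transform inputs directly.
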(event OnTrigger(triggerComponent)
  (Audio|PlaySound2D "/Game/Audio/Sounds/Intractibles/PressurePlate_Press.PressurePlate_Press" 1.0 1.0 0.0 0 0)
  (Utilities|FlowControl|Sequence
    (:then_0
      (Components|MoveComponentTo (Variables|Default|GetCollisionComponent) (Transformation|GetActorLocation (Variables|Default|GetTargetUp)) (Transformation|GetWorldRotation (Variables|Default|GetCollisionComponent)) false false 0.3 false) ; enters at Stop
    )
    (:then_1
      (Components|MoveComponentTo (Variables|Default|GetCollisionComponent) (Transformation|GetActorLocation (Variables|Default|GetTargetDown)) (Transformation|GetWorldRotation (Variables|Default|GetCollisionComponent)) false false 0.3 false))))

(event OnTriggerReverse(triggerComponent)
  (Audio|PlaySound2D "/Game/Audio/Sounds/Intractibles/PressurePlate_Release.PressurePlate_Release" 1.0 1.0 0.0 0 0)
  (Utilities|FlowControl|Sequence
    (:then_0
      (Components|MoveComponentTo (Variables|Default|GetCollisionComponent) (Transformation|GetActorLocation (Variables|Default|GetTargetDown)) (Transformation|GetWorldRotation (Variables|Default|GetCollisionComponent)) false false 0.3 false) ; enters at Stop
    )
    (:then_1
      (Components|MoveComponentTo (Variables|Default|GetCollisionComponent) (Transformation|GetActorLocation (Variables|Default|GetTargetUp)) (Transformation|GetWorldRotation (Variables|Default|GetCollisionComponent)) false false 0.3 false))))

(fn ConstructionScript)