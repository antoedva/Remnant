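; Puzzle receiver bookshelf for Room02 Puzzle01 that snaps between standing, laying-down and hovering poses when its BlueprintLink is triggered.
; On trigger, it checks whether rail bookshelves A and B sit at their mid targets to step NodeID forward or back along ReceiverTargets.
; An instant MoveComponentTo applies the selected target's transform.
; Attach, detach and rotation-check helpers exist but are not called here.
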(event OnTrigger(blueprintLink)
  (params (channel :type Integer))
  (bind _output (Utilities|GetNodeID))
  (bind _output_2 (Utilities|GetNodeID))
  (if (Math|Vector|NotEqual(Vector) (Transformation|GetActorLocation (Variables|Default|GetMovingBSRailB)) (Transformation|GetActorLocation (Variables|Default|GetMovingBSRailBTarget)) 5.0)
    (Development|PrintString "B Not In Middle")
    (if (CallFunction|IncrementID)
      (if (Math|Vector|NotEqual(Vector) (Transformation|GetActorLocation (Variables|Default|GetMovingBSRailA)) (Transformation|GetActorLocation (Variables|Default|GetMovingBSRailATarget)) 5.0)
        (Development|PrintString "Laying Down")
        ;[1 1 1] Increment Index and move BS
        (Components|MoveComponentTo (Variables|Default|GetDefaultSceneRoot) (Transformation|GetActorLocation _output) (Transformation|GetActorRotation _output) false false 0.0 false :!label _label)
        (elif (CallFunction|IncrementID)
          (Development|PrintString "Hover")
          (goto _label))))
    (elif (CallFunction|DecrementID)
      (Development|PrintString "Standing")
      ;[1 1 1] Decrement Index and move BS
      (Components|MoveComponentTo (Variables|Default|GetDefaultSceneRoot) (Transformation|GetActorLocation _output_2) (Transformation|GetActorRotation _output_2) false false 0.0 false))))

(event EventBeginPlay
  (bind _output_get (Variables|Default|SetNum%20Nodes (Utilities|Array|Length (Variables|/Script/Remnant.ReceiverTargets|Getreceiver_targets_ (Variables|Default|Gettargets_)))))
  (Math|Integer|DecrementInt _output_get))

(fn ConstructionScript)

(fn DecrementID
  (if (>= (- (Variables|Default|GetNode%20ID) 1) 0)
    (Math|Integer|DecrementInt (Variables|Default|GetNode%20ID)
      (:%20%20
        (return true)))
    (else
      (return false))))

(fn IncrementID
  (if (<= (+ (Variables|Default|GetNode%20ID) 1) (Variables|Default|GetNum%20Nodes))
    (Math|Integer|IncrementInt (Variables|Default|GetNode%20ID)
      (:%20%20
        (return true)))
    (else
      (return false))))

(fn AttachObject
  (bind _output (Utilities|GetNodeID))
  (if (== (Variables|Default|GetNode%20ID) (Variables|Default|GetNum%20Nodes))
    (Utilities|IsValid _output
      (:Is%20Valid
        (Transformation|AttachComponentToComponent (Variables|Default|GetDefaultSceneRoot) (Variables|/Script/Engine.Actor|GetRootComponent _output) "None" "SnapToTarget" "SnapToTarget" "KeepWorld" true)
        (return)))))

(fn TryDettachObject
  (Utilities|IsValid (Transformation|GetAttachParent (Variables|Default|GetDefaultSceneRoot))
    (:Is%20Valid
      (Transformation|DetachFromComponent (Variables|Default|GetDefaultSceneRoot) "KeepWorld" "KeepWorld" "KeepWorld" false)
      (return))
    (:Is%20Not%20Valid
      (return))))

(fn MoveAllowed
  (bind _defaultsceneroot (Variables|Default|GetDefaultSceneRoot))
  (bind _returnvalue (Transformation|GetAttachParent _defaultsceneroot))
  (Utilities|IsValid _returnvalue
    (:Is%20Valid
      (if (Math|Rotator|Equal(Rotator) (Transformation|GetWorldRotation (Transformation|GetAttachParent (Transformation|GetAttachParent _returnvalue))) "0, 0, 0" 0.0001)
        (return true)
        (else
          (return false))))
    (:Is%20Not%20Valid
      (return true))))

(fn IsCircleRotated
  (if (== (Variables|Default|GetNode%20ID) 2)
    (if (Utilities|Enum|NotEqual(Enum) (Transformation|GetActorRotation (Actor|GetAttachParentActor (Actor|GetAttachParentActor (Utilities|Array|Get(acopy) (Variables|/Script/Remnant.ReceiverTargets|Getreceiver_targets_ (Variables|Default|Gettargets_)) (+ (Variables|Default|GetNode%20ID) 1))))) "0, 0, 0")
      (return true)
      (else
        (return false)))
    (else
      (return false))))