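; Puzzle bookshelf for Room02 Puzzle01 that steps along a chain of receiver target nodes when triggered through BlueprintLink.
; Channel 0 advances and channel 1 goes back, moving instantly to each node's transform.
; It attaches to the last node on arrival and detaches when stepping back.
; Moves are refused when BlockActor occupies its target at the final link or when the node's parent circle is rotated away from zero.
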(event OnTrigger(blueprintLink)
  (params (channel :type Integer))
  (bind _output (Utilities|GetNodeID))
  (bind _output_2 (Utilities|GetNodeID))
  (bind _blockactor (Variables|Default|GetBlockActor))
  (bind _blockactortarget (Variables|Default|GetBlockActorTarget))
  (bind _returnvalue (Transformation|GetActorLocation _blockactor))
  (bind _returnvalue_2 (Transformation|GetActorLocation _blockactortarget))
  (bind _returnvalue_3 (Math|Vector|NotEqual(Vector) _returnvalue _returnvalue_2 5.0))
  (if (CallFunction|MoveAllowed)
    (switch int channel
      (:0
        (if (== (Variables|Default|GetNode%20ID) (- (Variables|Default|GetNum%20Nodes) 1))
          (if _returnvalue_3
            (if (not (CallFunction|IsCircleRotated)) :!label _label
              (if (CallFunction|IncrementID)
                (Components|MoveComponentTo (Variables|Default|GetDefaultSceneRoot) (Transformation|GetActorLocation _output) (Transformation|GetActorRotation _output) false false 0.0 false)
                (CallFunction|AttachObject))))
          (else
            (goto _label))))
      (:1
        (if (== (Variables|Default|GetNode%20ID) (Variables|Default|GetNum%20Nodes))
          (if _returnvalue_3
            (if (CallFunction|DecrementID) :!label _label_2
              (CallFunction|TryDettachObject)
              (Components|MoveComponentTo (Variables|Default|GetDefaultSceneRoot) (Transformation|GetActorLocation _output_2) (Transformation|GetActorRotation _output_2) false false 0.0 false)))
          (else
            (goto _label_2)))))))

(event EventBeginPlay
  (bind _output_get (Variables|Default|SetNum%20Nodes (Utilities|Array|Length (Variables|/Script/Remnant.ReceiverTargets|Getreceiver_targets_ (Variables|Default|Gettargets_)))))
  (Math|Integer|DecrementInt _output_get))

(fn ConstructionScript)

(fn DecrementID
  (if (>= (- (Variables|Default|GetNode%20ID) 1) 0)
    (Math|Integer|DecrementInt (Variables|Default|GetNode%20ID)
      (:%20%20
        (return true)))
    (else
      (return false))))

(fn IncrementID
  (if (<= (+ (Variables|Default|GetNode%20ID) 1) (Variables|Default|GetNum%20Nodes))
    (Math|Integer|IncrementInt (Variables|Default|GetNode%20ID)
      (:%20%20
        (return true)))
    (else
      (return false))))

(fn AttachObject
  (bind _output (Utilities|GetNodeID))
  (if (== (Variables|Default|GetNode%20ID) (Variables|Default|GetNum%20Nodes))
    (Utilities|IsValid _output
      (:Is%20Valid
        (Transformation|AttachComponentToComponent (Variables|Default|GetDefaultSceneRoot) (Variables|/Script/Engine.Actor|GetRootComponent _output) "None" "SnapToTarget" "SnapToTarget" "KeepWorld" true)
        (return)))))

(fn TryDettachObject
  (Utilities|IsValid (Transformation|GetAttachParent (Variables|Default|GetDefaultSceneRoot))
    (:Is%20Valid
      (Transformation|DetachFromComponent (Variables|Default|GetDefaultSceneRoot) "KeepWorld" "KeepWorld" "KeepWorld" false)
      (return))
    (:Is%20Not%20Valid
      (return))))

(fn MoveAllowed
  (bind _defaultsceneroot (Variables|Default|GetDefaultSceneRoot))
  (bind _returnvalue (Transformation|GetAttachParent _defaultsceneroot))
  (Utilities|IsValid _returnvalue
    (:Is%20Valid
      (if (Math|Rotator|Equal(Rotator) (Transformation|GetWorldRotation (Transformation|GetAttachParent (Transformation|GetAttachParent _returnvalue))) "0, 0, 0" 0.0001)
        (return true)
        (else
          (return false))))
    (:Is%20Not%20Valid
      (return true))))

(fn IsCircleRotated
  (if (== (Variables|Default|GetNode%20ID) 2)
    (if (Utilities|Enum|NotEqual(Enum) (Transformation|GetActorRotation (Actor|GetAttachParentActor (Actor|GetAttachParentActor (Utilities|Array|Get(acopy) (Variables|/Script/Remnant.ReceiverTargets|Getreceiver_targets_ (Variables|Default|Gettargets_)) (+ (Variables|Default|GetNode%20ID) 1))))) "0, 0, 0")
      (return true)
      (else
        (return false)))
    (else
      (return false))))