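; Middle circle bookshelf receiver for the Room02 Puzzle01 sliding-bookshelf puzzle, which jumps instantly between indexed target nodes when another receiver triggers.
; If rail B's bookshelf is off its target, it steps back up to two nodes; otherwise it steps forward, skipping one when rail A's bookshelf is on target.
; Helpers for attaching, detaching and rotation checks exist but go uncalled in this event graph, and the circle's rotation branch does nothing.
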(event OnAnotherReceiverTriggered(blueprintLink)
  (params (receiver :type Trigger%20Receiver%20Actor%20Object%20Reference) (channel :type Integer))
  (bind _targets_ (Variables|Default|Gettargets_))
  (bind _targets__2 (Variables|Default|Gettargets_))
  (bind _returnvalue (Class|ReceiverTargets|GetCurrentNode _targets_))
  (bind _returnvalue_2 (Class|ReceiverTargets|GetCurrentNode _targets__2))
  (bind _asbp_circle (Utilities|Casting|CastToBP_Circle (Variables|Default|GetTheCircle)))
  (if (Variables|/Game/Puzzles/Room02/Puzzle01/Receivers/Part03/BP_Circle.BP_Circle_C|GetIsRotated _asbp_circle)
    _
    (else
      _))
  (if (Math|Vector|NotEqual(Vector) (Transformation|GetActorLocation (Variables|Default|GetMovingBSRailB)) (Transformation|GetActorLocation (Variables|Default|GetMovingBSRailBTarget)) 5.0)
    (if (Class|ReceiverTargets|DecrementID (Variables|Default|Gettargets_))
      (if (Class|ReceiverTargets|DecrementID _targets_)
        _
        (else
          _))
      ;[1 1 1] Decrement Index and move BS
      (Components|MoveComponentTo (Variables|Default|GetDefaultSceneRoot) (Transformation|GetActorLocation _returnvalue) (Transformation|GetActorRotation _returnvalue) false false 0.0 false))
    (elif (Class|ReceiverTargets|IncrementID (Variables|Default|Gettargets_))
      (if (Math|Vector|NotEqual(Vector) (Transformation|GetActorLocation (Variables|Default|GetMovingBSRailA)) (Transformation|GetActorLocation (Variables|Default|GetMovingBSRailATarget)) 5.0)
        ;[1 1 1] Increment Index and move BS
        (Components|MoveComponentTo (Variables|Default|GetDefaultSceneRoot) (Transformation|GetActorLocation _returnvalue_2) (Transformation|GetActorRotation _returnvalue_2) false false 0.0 false :!label _label)
        (elif (Class|ReceiverTargets|IncrementID (Variables|Default|Gettargets_))
          (goto _label))))))

(fn ConstructionScript)

(fn DecrementID
  (if (>= (- (Variables|Default|GetNode%20ID) 1) 0)
    (Math|Integer|DecrementInt (Variables|Default|GetNode%20ID)
      (:%20%20
        (return true)))
    (else
      (return false))))

(fn IncrementID
  (if (<= (+ (Variables|Default|GetNode%20ID) 1) (Variables|Default|GetNum%20Nodes))
    (Math|Integer|IncrementInt (Variables|Default|GetNode%20ID)
      (:%20%20
        (return true)))
    (else
      (return false))))

(fn AttachObject
  (bind _output (Utilities|GetNodeID))
  (if (== (Variables|Default|GetNode%20ID) (Variables|Default|GetNum%20Nodes))
    (Utilities|IsValid _output
      (:Is%20Valid
        (Transformation|AttachComponentToComponent (Variables|Default|GetDefaultSceneRoot) (Variables|/Script/Engine.Actor|GetRootComponent _output) "None" "SnapToTarget" "SnapToTarget" "KeepWorld" true)
        (return)))))

(fn TryDettachObject
  (Utilities|IsValid (Transformation|GetAttachParent (Variables|Default|GetDefaultSceneRoot))
    (:Is%20Valid
      (Transformation|DetachFromComponent (Variables|Default|GetDefaultSceneRoot) "KeepWorld" "KeepWorld" "KeepWorld" false)
      (return))
    (:Is%20Not%20Valid
      (return))))

(fn MoveAllowed
  (bind _defaultsceneroot (Variables|Default|GetDefaultSceneRoot))
  (bind _returnvalue (Transformation|GetAttachParent _defaultsceneroot))
  (Utilities|IsValid _returnvalue
    (:Is%20Valid
      (if (Math|Rotator|Equal(Rotator) (Transformation|GetWorldRotation (Transformation|GetAttachParent (Transformation|GetAttachParent _returnvalue))) "0, 0, 0" 0.0001)
        (return true)
        (else
          (return false))))
    (:Is%20Not%20Valid
      (return true))))

(fn IsCircleRotated
  (if (== (Variables|Default|GetNode%20ID) 2)
    (if (Utilities|Enum|NotEqual(Enum) (Transformation|GetActorRotation (Actor|GetAttachParentActor (Actor|GetAttachParentActor (Utilities|Array|Get(acopy) (Variables|/Script/Remnant.ReceiverTargets|Getreceiver_targets_ (Variables|Default|Gettargets_)) (+ (Variables|Default|GetNode%20ID) 1))))) "0, 0, 0")
      (return true)
      (else
        (return false)))
    (else
      (return false))))