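; Puzzle circle receiver in Room02 that alternates between rotating 90 degrees and back on each channel 0 BlueprintLink trigger.
; On rotating out, a match between actors attached to AttachedTargetPoints and ActorsToCheck instantly rotates EndDoor, sets IsRotated and triggers three linked receivers.
; Rotating back clears IsRotated and triggers those receivers, leaving the door as is.
; The loop that fills AttachedTargetPoints from attached actors is never run.
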(event OnTrigger(blueprintLink)
  (params (channel :type Integer))
  (bind _defaultsceneroot (Variables|Default|GetDefaultSceneRoot))
  (bind _defaultsceneroot_2 (Variables|Default|GetDefaultSceneRoot))
  (bind _end_door (Variables|Default|GetEnd%20door))
  (bind _rootcomponent (Variables|/Script/Engine.Actor|GetRootComponent _end_door))
  (switch int channel
    (:0
      (Utilities|FlowControl|FlipFlop
        (:A
          (Components|MoveComponentTo _defaultsceneroot_2 (Transformation|GetWorldLocation _defaultsceneroot_2) "0,90.000000, 0" false false 3.0 false)
          (for _array_element (Variables|Default|GetAttachedTargetPoints)
            (for _array_element_2 (Actor|GetAttachedActors _array_element)
              (Utilities|IsValid _array_element_2
                (:Is%20Valid
                  (for _array_element_3 (Variables|Default|GetActorsToCheck)
                    (if (== _array_element_3 _array_element_2)
                      (Components|MoveComponentTo _rootcomponent (Transformation|GetWorldLocation _rootcomponent) "0, 0,-90.000000" false false 0.0 false)
                      (Variables|Default|SetIsRotated true)
                      (Class|TriggerReceiverActor|TriggerAnotherReceiver 0 (Variables|Default|GetLinkReceiver))
                      (Class|TriggerReceiverActor|TriggerAnotherReceiver 0 (Variables|Default|GetLinkReceiver2))
                      (Class|TriggerReceiverActor|TriggerAnotherReceiver 0 (Variables|Default|GetLinkReceiver3)))))))))
        (:B
          (Components|MoveComponentTo _defaultsceneroot (Transformation|GetWorldLocation _defaultsceneroot) "0, 0, 0" false false 3.0 false)
          (Variables|Default|SetIsRotated false)
          (Class|TriggerReceiverActor|TriggerAnotherReceiver 0 (Variables|Default|GetLinkReceiver))
          (Class|TriggerReceiverActor|TriggerAnotherReceiver 0 (Variables|Default|GetLinkReceiver2))
          (Class|TriggerReceiverActor|TriggerAnotherReceiver 0 (Variables|Default|GetLinkReceiver3)))))))

(event EventBeginPlay)

(fn ConstructionScript)