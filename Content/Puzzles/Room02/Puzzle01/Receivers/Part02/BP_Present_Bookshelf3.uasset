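; Bookshelf puzzle receiver in Room02 that moves to the next target node, then slowly back to the previous one.
; BlueprintLink channel 1 starts the trip when ready, stepping NodeID through the ReceiverTargets actors; channels 10 and 11 pause and resume it.
; Timelines act as clocks for each leg, so MoveComponentTo restarts with only the remaining time after a pause.
; Ready is restored once the return move completes.
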(event OnTrigger(blueprintLink)
  (params (channel :type Integer))
  (bind _node_id (Variables|Default|GetNode%20ID))
  (bind _num_nodes (Variables|Default|GetNum%20Nodes))
  (bind _returnvalue (== _node_id _num_nodes))
  (switch int channel
    (:1
      (if (Variables|Default|GetReady)
        (Variables|Default|SetReady false)
        (if (CallFunction|IncrementID)
          (bind _time (Timeline|Timeline_1 PlayFromStart)
            (:Update
              (Variables|Default|SetElapsed%20Time _time)
              (Utilities|FlowControl|DoOnce false :!label _label
                (:Completed
                  (Components|MoveComponentTo (Variables|Default|GetDefaultSceneRoot) (Transformation|GetActorLocation (Utilities|GetNodeID)) (Transformation|GetWorldRotation (Variables|Default|GetDefaultSceneRoot)) false false (- 3.0 (Variables|Default|GetElapsed%20Time)) false :!label _label_2)
                  (goto _label Reset))))
            (:Finished
              (if (CallFunction|DecrementID)
                (bind _time_2 (Timeline|Timeline_0 PlayFromStart)
                  (:Update
                    (Variables|Default|SetElapsed%20Time _time_2)
                    (Utilities|FlowControl|DoOnce false :!label _label_3
                      (:Completed
                        (Components|MoveComponentTo (Variables|Default|GetDefaultSceneRoot) (Transformation|GetActorLocation (Utilities|GetNodeID)) (Transformation|GetWorldRotation (Variables|Default|GetDefaultSceneRoot)) false false (- 1e+01 (Variables|Default|GetElapsed%20Time)) false :!label _label_4)
                        (Utilities|FlowControl|Sequence
                          (:then_0
                            (goto _label_3 Reset))
                          (:then_1
                            (Variables|Default|SetReady true)))))))))))))
    (:10
      (if _returnvalue
        (Utilities|FlowControl|Sequence
          (:then_0
            (Timeline|Timeline_1 Stop))
          (:then_1
            (goto _label Reset))
          (:then_2
            (goto _label_2 Stop)))
        (else
          (Utilities|FlowControl|Sequence
            (:then_0
              (Timeline|Timeline_0 Stop))
            (:then_1
              (goto _label_3 Reset))
            (:then_2
              (goto _label_4 Stop))))))
    (:11
      (if _returnvalue
        (Timeline|Timeline_1 Play)
        (else
          (Timeline|Timeline_0 Play))))))

(event EventBeginPlay
  (bind _output_get (Variables|Default|SetNum%20Nodes (Utilities|Array|Length (Variables|/Script/Remnant.ReceiverTargets|Getreceiver_targets_ (Variables|Default|Gettargets_)))))
  (Math|Integer|DecrementInt _output_get))

(fn ConstructionScript)

(fn DecrementID
  (if (>= (- (Variables|Default|GetNode%20ID) 1) 0)
    (Math|Integer|DecrementInt (Variables|Default|GetNode%20ID)
      (:%20%20
        (return true)))
    (else
      (return false))))

(fn IncrementID
  (if (<= (+ (Variables|Default|GetNode%20ID) 1) (Variables|Default|GetNum%20Nodes))
    (Math|Integer|IncrementInt (Variables|Default|GetNode%20ID)
      (:%20%20
        (return true)))
    (else
      (return false))))