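; Puzzle button for Room02 Puzzle01, named for rotating a circle, that gives press feedback when triggered; no rotation logic appears here.
; BeginPlay creates a dynamic material on PastButton with its emissive glow off.
; TriggerComponent's OnTrigger lights the glow, moves the Parent component down, waits briefly, raises it, then switches the glow off again.
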(event OnTrigger(triggerComponent)
  (Utilities|FlowControl|Sequence
    (:then_0
      (Rendering|Material|SetScalarParameterValue (stale EventBeginPlay _returnvalue) "Emissive_intensity" (Variables|Default|GetEmissive) :!class /Script/Engine.MaterialInstanceDynamic))
    (:then_1
      (Components|MoveComponentTo (Variables|Default|GetParent) "0,0.000000,-2.000000" "0, 0, 0" false false 0.2 false)
      (Utilities|FlowControl|Delay 0.5)
      (Components|MoveComponentTo (Variables|Default|GetParent) "0, 0,2.000000" "0, 0, 0" false false 0.2 false)
      (Rendering|Material|SetScalarParameterValue (stale EventBeginPlay _returnvalue) "Emissive_intensity" 0.0 :!class /Script/Engine.MaterialInstanceDynamic))))

(event EventBeginPlay
  (bind _past_button (Variables|Default|GetPast_Button))
  (Utilities|FlowControl|Sequence
    (:then_0
      (bind _returnvalue (Rendering|Material|CreateDynamicMaterialInstance _past_button 0 (Rendering|Material|GetMaterial _past_button 0) "None" :!class /Script/Engine.PrimitiveComponent))
      (Rendering|Material|SetScalarParameterValue _returnvalue "Emissive_intensity" 0.0 :!class /Script/Engine.MaterialInstanceDynamic))
    (:then_1
      (|CallParentFunction))))

(event Collision|EventActorBeginOverlap
  (params (OtherActor :type Actor%20Object%20Reference))
  (|CallParentFunction OtherActor) ; This node is disabled and will not be called.\nDrag off pins to build functionality.
)

(event EventTick
  (params (DeltaSeconds :type Float%20%28single-precision%29))
  (|CallParentFunction DeltaSeconds) ; This node is disabled and will not be called.\nDrag off pins to build functionality.
)

(fn ConstructionScript
  (|CallParentFunction))