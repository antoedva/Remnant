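; Moving stair for the Library level that responds to two BlueprintLink trigger channels.
; When both channels are triggered, it eases to the position and rotation of the second receiver target actor.
; A reverse trigger on either channel clears that flag and moves it faster to the first target, provided that channel's counter can decrement.
; Debug prints remain, and the Tick check does nothing.
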(event OnTrigger(blueprintLink)
  (params (channel :type Integer))
  (bind _startactor (Variables|Default|GetStartActor))
  (switch int channel
    (:0
      (Math|Integer|IncrementInt (Variables|Default|GetCounter1)
        (:%20%20
          (bind _output_get (Variables|Default|SetTrigger1 true)))))
    (:1
      (Math|Integer|IncrementInt (Variables|Default|GetCounter2)
        (:%20%20
          (bind _output_get_2 (Variables|Default|SetTrigger%202 true))))))
  (if (and _output_get _output_get_2)
    (Development|PrintString "true")
    (Components|MoveComponentTo (Variables|Transformation|GetRootComponent) (Transformation|GetActorLocation _startactor) (Transformation|GetActorRotation _startactor) true true 2.0 false)))

(event OnTriggerReverse(blueprintLink)
  (params (channel :type Integer))
  (bind _endactor (Variables|Default|GetEndActor))
  (switch int channel
    (:0
      (if (CallFunction|Decrement (Variables|Default|GetCounter1))
        (Variables|Default|SetTrigger1 false)
        (Development|PrintString "false" :!label _label)
        (Components|MoveComponentTo (Variables|Transformation|GetRootComponent) (Transformation|GetActorLocation _endactor) (Transformation|GetActorRotation _endactor) false false 1.0 false)))
    (:1
      (if (CallFunction|Decrement (Variables|Default|GetCounter2))
        (Variables|Default|SetTrigger%202 false)
        (goto _label)))))

(event EventTick
  (params (DeltaSeconds :type Float%20%28single-precision%29))
  (if (or (<= (Variables|Default|GetCounter1) 0) (<= (Variables|Default|GetCounter2) 0))
    _))

(event EventBeginPlay
  (bind _targets_ (Variables|Default|Gettargets_))
  (bind _receiver_targets_ (Variables|/Script/Remnant.ReceiverTargets|Getreceiver_targets_ _targets_))
  (Variables|Default|SetStartActor (Utilities|Array|Get(acopy) _receiver_targets_ 1))
  (Variables|Default|SetEndActor (Utilities|Array|Get(acopy) _receiver_targets_)))

(fn ConstructionScript)

(fn Decrement
  (params (Counter :type Integer))
  (if (>= (- Counter 1) 0)
    (Math|Integer|DecrementInt Counter
      (:%20%20
        (return true)))
    (else
      (return false))))