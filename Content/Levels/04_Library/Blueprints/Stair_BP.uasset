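; Library level stair that moves between two target actors in response to BlueprintLink trigger channels.
; Channels 0 and 1 must both be triggered to ease it to the start actor; a successfully decremented reverse trigger on either sends it to the end actor.
; Channels 10 and 11 control stopping and resuming those MoveComponentTo moves.
; An older Timeline-based node-stepping event is marked unused, and Tick does nothing.
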(event OnTriggerReverse(blueprintLink)
  (params (channel :type Integer))
  (bind _endactor (Variables|Default|GetEndActor))
  (switch int channel
    (:0
      (if (CallFunction|DecrementCounter (Variables|Default|GetCounter1))
        (Variables|Default|SetTrigger1 false)
        (Development|PrintString "false" :!label _label)
        (Components|MoveComponentTo (Variables|Transformation|GetRootComponent) (Transformation|GetActorLocation _endactor) (Transformation|GetActorRotation _endactor) false false 1.0 false :!label _label_2)))
    (:1
      (if (CallFunction|DecrementCounter (Variables|Default|GetCounter2))
        (Variables|Default|SetTrigger%202 false)
        (goto _label)))
    (:10
      (goto _label_2 Stop))
    (:11
      (goto _label_2))))

(event OnTrigger(blueprintLink)
  (params (channel :type Integer))
  (bind _startactor (Variables|Default|GetStartActor))
  (switch int channel
    (:0
      (Math|Integer|IncrementInt (Variables|Default|GetCounter1)
        (:%20%20
          (bind _output_get (Variables|Default|SetTrigger1 true))
          (if (and _output_get (stale _output_get_2)) :!label _label
            (Development|PrintString "true")
            (Components|MoveComponentTo (Variables|Transformation|GetRootComponent) (Transformation|GetActorLocation _startactor) (Transformation|GetActorRotation _startactor) true true 2.0 false :!label _label_2)))))
    (:1
      (Math|Integer|IncrementInt (Variables|Default|GetCounter2)
        (:%20%20
          (bind _output_get_2 (Variables|Default|SetTrigger%202 true))
          (goto _label))))
    (:10
      (goto _label_2 Stop))
    (:11
      (goto _label_2))))

(event Custom|CustomEvent
  (params (channel :type Integer))
  (bind _node_id (Variables|Default|GetNode%20ID))
  (bind _num_nodes (Variables|Default|GetNum%20Nodes))
  (bind _returnvalue (== _node_id _num_nodes))
  ;[1 1 1] NOT IN USE
  (switch int channel
    (:0
      (if (Variables|Default|GetReady)
        (Variables|Default|SetReady false)
        (if (CallFunction|IncrementID)
          (bind _newtrack_1 (Timeline|Timeline_1 PlayFromStart)
            (:Update
              (Variables|Default|SetElapsed%20Time _newtrack_1)
              (Utilities|FlowControl|DoOnce false :!label _label
                (:Completed
                  (Components|MoveComponentTo (Variables|Default|GetDefaultSceneRoot) (Transformation|GetActorLocation) (Transformation|GetWorldRotation (Variables|Default|GetDefaultSceneRoot)) false false (- 3.0 (Variables|Default|GetElapsed%20Time)) false :!label _label_2)
                  (goto _label Reset))))
            (:Finished
              (if (CallFunction|DecrementCounter)
                (bind _newtrack_1_2 (Timeline|Timeline_0 PlayFromStart)
                  (:Update
                    (Variables|Default|SetElapsed%20Time _newtrack_1_2)
                    (Utilities|FlowControl|DoOnce false :!label _label_3
                      (:Completed
                        (Components|MoveComponentTo (Variables|Default|GetDefaultSceneRoot) (Transformation|GetActorLocation) (Transformation|GetWorldRotation (Variables|Default|GetDefaultSceneRoot)) false false (- 1e+01 (Variables|Default|GetElapsed%20Time)) false :!label _label_4)
                        (Utilities|FlowControl|Sequence
                          (:then_0
                            (goto _label_3 Reset))
                          (:then_1
                            (Variables|Default|SetReady true)))))))))))))
    (:10
      (if _returnvalue
        (Utilities|FlowControl|Sequence
          (:then_0
            (Timeline|Timeline_1 Stop))
          (:then_1
            (goto _label Reset))
          (:then_2
            (goto _label_2 Stop)))
        (else
          (Utilities|FlowControl|Sequence
            (:then_0
              (Timeline|Timeline_0 Stop))
            (:then_1
              (goto _label_3 Reset))
            (:then_2
              (goto _label_4 Stop))))))
    (:11
      (if _returnvalue
        (Timeline|Timeline_1 Play)
        (else
          (Timeline|Timeline_0 Play))))))

(event EventTick
  (params (DeltaSeconds :type Float%20%28single-precision%29))
  (if (or (<= (Variables|Default|GetCounter1) 0) (<= (Variables|Default|GetCounter2) 0))
    _))

(event EventBeginPlay
  (bind _targets_ (Variables|Default|Gettargets_))
  (bind _receiver_targets_ (Variables|/Script/Remnant.ReceiverTargets|Getreceiver_targets_ _targets_))
  (Variables|Default|SetStartActor (Utilities|Array|Get(acopy) _receiver_targets_ 1))
  (Variables|Default|SetEndActor (Utilities|Array|Get(acopy) _receiver_targets_)))

(fn ConstructionScript)

(fn DecrementCounter
  (params (Counter :type Integer))
  (if (>= (- Counter 1) 0)
    (Math|Integer|DecrementInt Counter
      (:%20%20
        (return true)))
    (else
      (return false))))

(fn IncrementID
  (if (<= (+ (Variables|Default|GetNode%20ID) 1) (Variables|Default|GetNum%20Nodes))
    (Math|Integer|IncrementInt (Variables|Default|GetNode%20ID)
      (:%20%20
        (return true)))
    (else
      (return false))))