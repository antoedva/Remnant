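; Library-level stair actor, apparently an older version, that rises once its BlueprintLink has been triggered at least twice.
; Each trigger increments a clamped counter and prints it for debugging.
; From the second trigger onward, MoveComponentTo eases the root upward by a fixed offset from its current world position, so further triggers raise it again.
; Reverse triggers do nothing, and StairZ is unused.
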(event OnTrigger(blueprintLink)
  (params (channel :type Integer))
  (Variables|Default|Setcounter_test (+ (Math|Integer|Clamp(Integer) (Variables|Default|Getcounter_test) 0 2) 1))
  (Development|PrintString (Utilities|String|ToString(Integer) (Math|Integer|Clamp(Integer) (Variables|Default|Getcounter_test) 0 2)))
  (if (>= (Math|Integer|Clamp(Integer) (Variables|Default|Getcounter_test) 0 2) 2)
    (Components|MoveComponentTo (Variables|Transformation|GetRootComponent) (+ (Transformation|GetWorldLocation (Variables|Transformation|GetRootComponent)) (Math|Vector|MakeVector 0.0 0.0 4e+02)) (Transformation|GetWorldRotation (Variables|Default|GetDefaultSceneRoot)) true true 2.0 false)))

(event OnTriggerReverse(blueprintLink)
  (params (channel :type Integer)))

(fn ConstructionScript)