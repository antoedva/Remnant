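; Library corridor door that slides between two positions taken from receiver target actors, driven by BlueprintLink triggers.
; Channel 0 moves it to the end position, while a reverse trigger returns it to the start after a short delay.
; If the trigger reverses during opening, completion of that move also schedules the return.
; Channels 10 and 11 set a Frozen flag and stop or restart both moves.
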(event OnTrigger(blueprintLink)
  (params (channel :type Integer))
  (switch int channel
    (:0
      (Variables|Default|SetIs_Inside true)
      (Components|MoveComponentTo (Variables|Transformation|GetRootComponent) (Variables|Default|GetEndPos) "0, 0,0.000000" false false 0.5 false :!label _label)
      (if (not (Variables|Default|GetIs_Inside))
        (Utilities|FlowControl|Delay 2.0)
        (Components|MoveComponentTo (Variables|Transformation|GetRootComponent) (Variables|Default|GetStartPos) "0, 0, 0" false false 0.5 false :!label _label_2)))
    (:10
      (Variables|Default|SetFrozen true)
      (Utilities|FlowControl|Sequence
        (:then_0
          (goto _label Stop))
        (:then_1
          (goto _label_2 Stop))))
    (:11
      (Variables|Default|SetFrozen false)
      (Utilities|FlowControl|Sequence
        (:then_0
          (goto _label))
        (:then_1
          (goto _label_2))))))

(event OnTriggerReverse(blueprintLink)
  (params (channel :type Integer))
  (Variables|Default|SetIs_Inside false)
  (Utilities|FlowControl|Delay 2.0)
  (Components|MoveComponentTo (Variables|Transformation|GetRootComponent) (Variables|Default|GetStartPos) "0, 0, 0" false false 0.5 false))

(event EventBeginPlay
  (bind _targets_ (Variables|Default|Gettargets_))
  (bind _receiver_targets_ (Variables|/Script/Remnant.ReceiverTargets|Getreceiver_targets_ _targets_))
  (Variables|Default|SetStartPos (Transformation|GetActorLocation (Utilities|Array|Get(acopy) _receiver_targets_ 1)))
  (Variables|Default|SetEndPos (Transformation|GetActorLocation (Utilities|Array|Get(acopy) _receiver_targets_))))

(fn ConstructionScript)